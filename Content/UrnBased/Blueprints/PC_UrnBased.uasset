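; Player controller for the UrnBased game that pans the camera by moving the player pawn along world X and Y.
; The MoveForward and MoveRight axis events check only the input's sign and shift the pawn's location by a fixed step without sweeping.
; Movement ignores axis magnitude, pawn rotation and delta time, so pan speed depends on frame rate.
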(event `InputAxis|MoveForward`
  (params (AxisValue :type "Float (single-precision)"))
  (bind _returnvalue (`GameplayStatics.GetPlayerPawn` 0))
  (bind _returnvalue_2 (`self.K2_GetActorLocation` _returnvalue))
  ;[1 1 1] Camera move up and down
  (if (> AxisValue 0.0)
    (`self.K2_SetActorLocation` _returnvalue (+ _returnvalue_2 (5.0 0.0 0.0)) false)
    (elif (< AxisValue 0.0)
      (`self.K2_SetActorLocation` _returnvalue (- _returnvalue_2 (5.0 0.0 0.0)) false))))

(event `InputAxis|MoveRight`
  (params (AxisValue :type "Float (single-precision)"))
  (bind _returnvalue (`GameplayStatics.GetPlayerPawn` 0))
  (bind _returnvalue_2 (`self.K2_GetActorLocation` _returnvalue))
  ;[1 1 1] Camera move right and left
  (if (> AxisValue 0.0)
    (`self.K2_SetActorLocation` _returnvalue (+ _returnvalue_2 (0.0 5.0 0.0)) false)
    (elif (< AxisValue 0.0)
      (`self.K2_SetActorLocation` _returnvalue (- _returnvalue_2 (0.0 5.0 0.0)) false))))

(fn `UserConstructionScript`)