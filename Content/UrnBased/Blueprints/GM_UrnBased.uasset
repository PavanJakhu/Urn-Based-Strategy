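; GM_UrnBased is a game mode that holds the selected unit and tile and handles moving units across tiles.
; Selecting a unit caches its location and moves the player pawn to its X/Y, keeping the pawn's height.
; Selecting a tile moves the unit only if that tile is in its TilesAround list, then prints their horizontal distance in 50-unit steps.
; Getters and a direct location setter expose the selection state.
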(fn ConstructionScript)

(fn SetSelectedUnit
  (params (selectUnit :type Unit%20Object%20Reference))
  (bind _returnvalue (Game|Player|GetPlayerPawn 0))
  (bind _output_get (Variables|Default|SetSelectedUnit selectUnit))
  (bind _output_get_2 (Variables|Default|SetSelectedUnitOriginalLocation (Transformation|GetActorLocation _output_get)))
  (Transformation|SetActorLocation _returnvalue (Math|Vector|MakeVector (.x _output_get_2) (.y _output_get_2) (.z (Transformation|GetActorLocation _returnvalue))) false false))

(fn GetSelectedUnit
  (return (Variables|Default|GetSelectedUnit)))

(fn GetSelectedUnitLocaiton
  (return (Variables|Default|GetSelectedUnitOriginalLocation)))

(fn SetSelectedTile
  (params (selectedTile :type Tile%20Object%20Reference))
  (bind _selectedunit (Variables|Default|GetSelectedUnit))
  (bind _output_get (Variables|Default|SetSelectedTile selectedTile))
  (if (!= _output_get 0)
    (bind _array_element (Utilities|Array|ForEachLoopwithBreak (Variables|/Game/UrnBased/Blueprints/Units/Unit.Unit_C|GettilesAround _selectedunit) :!label _label)
      (:LoopBody
        (if (== _array_element _output_get)
          (Default|MoveUnitto _selectedunit (Transformation|GetActorLocation _output_get))
          (Development|PrintString (Utilities|String|ToString(Float) (/ (|(value-(value%50)) (Transformation|GetHorizontalDistanceTo _output_get _selectedunit)) 5e+01)))
          (goto _label Break))))))

(fn SetSelectedUnitLocation
  (params (newLocation :type Vector))
  (Transformation|SetActorLocation (Variables|Default|GetSelectedUnit) newLocation false false))

(fn GetSelectedTile
  (return (Variables|Default|GetSelectedTile)))