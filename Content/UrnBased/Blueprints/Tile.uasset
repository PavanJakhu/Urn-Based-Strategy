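; Clickable tile actor for the UrnBased game mode, with a terrain type of grass, dirt, snow or stone.
; The construction script sets the cube's material from the tile type.
; On click, the tile passes itself to GM_UrnBased as the selected tile.
; Disconnected timeline logic for sliding the selected unit between positions remains in the graph but never runs.
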(event `self.ReceiveActorOnClicked`
  (bind _asgm_urn_based (cast `/Game/UrnBased/Blueprints/GM_UrnBased` (`GameplayStatics.GetGameMode`)))
  (`/Game/UrnBased/Blueprints/GM_UrnBased.SetSelectedTile` _asgm_urn_based self))

(event `self.ReceiveBeginPlay`)

(event `self.ReceiveActorBeginOverlap`
  (params (OtherActor :type "Actor Object Reference")))

(event `self.ReceiveTick`
  (params (DeltaSeconds :type "Float (single-precision)")))

(fn `UserConstructionScript`
  (bind _cube (`self.Cube`))
  (switch `/Game/UrnBased/Blueprints/TileTypes` (`self.myTileType`)
    (:`NewEnumerator0`
      (`PrimitiveComponent.SetMaterial` _cube 0 "/Game/UrnBased/Materials/M_GrassTile.M_GrassTile"))
    (:`NewEnumerator1`
      (`PrimitiveComponent.SetMaterial` _cube 0 "/Game/UrnBased/Materials/M_DirtTile.M_DirtTile"))
    (:`NewEnumerator2`
      (`PrimitiveComponent.SetMaterial` _cube 0 "/Game/UrnBased/Materials/M_SnowTile.M_SnowTile"))
    (:`NewEnumerator3`
      (`PrimitiveComponent.SetMaterial` _cube 0 "/Game/UrnBased/Materials/M_StoneTile.M_StoneTile"))))