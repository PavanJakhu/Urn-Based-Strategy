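; Turn-based tactics unit with a stats struct and team-colored material, offering Move, Attack and Defend actions.
; Clicking it registers it as GM_UrnBased's selected unit, first triggering the previous selection's attack if this unit is targetable.
; Move highlights tiles found by sphere overlap using custom depth, with AI MoveTo handling travel.
; Attack sphere-traces units in range as targetable, while Defend doubles endurance until OnTurnBegin halves it.
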(event Custom|MoveUnitTo
  (params (Location :type Vector))
  (switch Utilities|FlowControl|Switch|SwitchonUnitStates (Variables|Default|GetmyState)
    (:NewEnumerator0
      (AI|AIMoveTo self Location 0 5.0 false))))

(event EventBeginPlay
  (Components|Activation|SetActive (Variables|Default|GetSphere) false false))

(event MouseInput|EventActorOnClicked
  (Utilities|FlowControl|Sequence
    (:then_0
      (if (Variables|Default|GetcanBeTargetted)
        (bind _asgm_urn_based (Utilities|Casting|CastToGM_UrnBased (Game|GetGameMode)))
        (bind _selectedunit (Default|GetSelectedUnit _asgm_urn_based))
        (Variables|Unit_C|SettargetUnit _selectedunit self)
        (CallFunction|Attack _selectedunit)))
    (:then_1
      (bind _asgm_urn_based_2 (Utilities|Casting|CastToGM_UrnBased (Game|GetGameMode)))
      (bind _selectedunit_2 (Default|GetSelectedUnit _asgm_urn_based_2))
      (if (!= _selectedunit_2 0)
        (bind _tiles (CallFunction|GetTilesAround _selectedunit_2 (+ (Math|Conversions|ToFloat(Integer) (Variables|/Script/Urn_Based.UrnUnit|Getspeed _selectedunit_2)) 1.0) (Transformation|GetActorLocation _selectedunit_2)))
        (for _array_element _tiles
          (Rendering|SetRenderCustomDepth (Variables|/Game/UrnBased/Blueprints/Tile.Tile_C|GetCube _array_element) false)))
      (Default|SetSelectedUnit _asgm_urn_based_2 self))))

(fn ConstructionScript
  (bind _cylinder (Variables|Default|GetCylinder))
  (Class|UrnUnit|SetStartingStats 10 3 3 10 10 10 10 10 10 10 10 3 1)
  (Variables|Default|SetmyStats (Utilities|Struct|MakeUnitStats 10 10 3 3 3 20 20 10 10 10 10 10 10 10 10 3 2))
  (switch Utilities|FlowControl|Switch|SwitchonTeamColours (Variables|Default|GetmyTeam)
    (:NewEnumerator0
      (Rendering|Material|SetMaterial _cylinder 0 "/Game/StarterContent/Materials/M_Metal_Rust.M_Metal_Rust"))
    (:NewEnumerator1
      (Rendering|Material|SetMaterial _cylinder 0 "/Game/StarterContent/Materials/M_Water_Lake.M_Water_Lake"))
    (:NewEnumerator2
      (Rendering|Material|SetMaterial _cylinder 0 "/Game/StarterContent/Materials/M_Ground_Grass.M_Ground_Grass"))))

(fn GetMyStats
  (return (Variables|Default|GetmyStats)))

(fn OnAttackClicked
  (bind _returnvalue (Transformation|GetActorLocation))
  (bind _mystats (Variables|Default|GetmyStats))
  (bind _returnvalue_2 (* (.range _mystats) 1e+02))
  (Variables|Default|SetmyState "NewEnumerator1")
  (Development|PrintString "AttackClicked")
  (Rendering|Debug|DrawDebugSphere _returnvalue _returnvalue_2 24 "(R=1.000000,G=0.000000,B=0.000000,A=1.000000)" 5.0)
  (bind _outhits (Collision|MultiSphereTraceForObjects _returnvalue _returnvalue _returnvalue_2 (Utilities|Array|MakeArray "ObjectTypeQuery3") false 0 "None"))
  (for _array_element _outhits
    (bind _asunit (Utilities|Casting|CastToUnit (.hitactor _array_element)))
    (CallFunction|SetCanbeTargetted _asunit true)))

(fn Attack
  (Class|UrnUnit|CalculateDamageTaken (Variables|Default|GettargetUnit) (Utilities|Struct|MakeAttackInfo "ATT_MELEE" 10)))

(fn SetCanbeTargetted
  (params (canBeTarget :type Boolean))
  (Variables|Default|SetcanBeTargetted canBeTarget))

(fn OnDefendClicked
  (Variables|Default|SetmyState "NewEnumerator3")
  (Development|PrintString "Set Active Pawn's Endurance to x 2 until it is active again")
  (Variables|Default|SetwasDefending true)
  (Variables|Default|SetmyStats (Utilities|Struct|MakeUnitStats (.hitpoints (Variables|Default|GetmyStats)) (.maxhitpoints (Variables|Default|GetmyStats)) (.speed (Variables|Default|GetmyStats)) (.actionpoints (Variables|Default|GetmyStats)) (.maxactionpoints (Variables|Default|GetmyStats)) (.powerpoints (Variables|Default|GetmyStats)) (.maxpowerpoints (Variables|Default|GetmyStats)) (.prowess (Variables|Default|GetmyStats)) (.accuracy (Variables|Default|GetmyStats)) (.strength (Variables|Default|GetmyStats)) (* (.endurance (Variables|Default|GetmyStats)) 2) (.agility (Variables|Default|GetmyStats)) (.willpower (Variables|Default|GetmyStats)) (.intelligence (Variables|Default|GetmyStats)) (.armour (Variables|Default|GetmyStats)) (.size (Variables|Default|GetmyStats)) (.range (Variables|Default|GetmyStats)))))

(fn OnTurnBegin
  (if (Variables|Default|GetwasDefending)
    (Variables|Default|SetwasDefending false)
    (Variables|Default|SetmyStats (Utilities|Struct|MakeUnitStats (.hitpoints (Variables|Default|GetmyStats)) (.maxhitpoints (Variables|Default|GetmyStats)) (.speed (Variables|Default|GetmyStats)) (.actionpoints (Variables|Default|GetmyStats)) (.maxactionpoints (Variables|Default|GetmyStats)) (.powerpoints (Variables|Default|GetmyStats)) (.maxpowerpoints (Variables|Default|GetmyStats)) (.prowess (Variables|Default|GetmyStats)) (.accuracy (Variables|Default|GetmyStats)) (.strength (Variables|Default|GetmyStats)) (/ (.endurance (Variables|Default|GetmyStats)) 2) (.agility (Variables|Default|GetmyStats)) (.willpower (Variables|Default|GetmyStats)) (.intelligence (Variables|Default|GetmyStats)) (.armour (Variables|Default|GetmyStats)) (.size (Variables|Default|GetmyStats)) (.range (Variables|Default|GetmyStats))))))

(fn OnTurnEnd)

(fn OnMoveClicked
  (Variables|Default|SetmyState "NewEnumerator0")
  (Development|PrintString "OnMoveClicked")
  (bind _asgm_urn_based (Utilities|Casting|CastToGM_UrnBased (Game|GetGameMode)))
  (bind _selectedunit (Default|GetSelectedUnit _asgm_urn_based))
  (bind _tiles (CallFunction|GetTilesAround _selectedunit (+ (Math|Conversions|ToFloat(Integer) (Variables|/Script/Urn_Based.UrnUnit|Getspeed _selectedunit)) 1.0) (Transformation|GetActorLocation _selectedunit)))
  (for _array_element _tiles
    (Rendering|SetRenderCustomDepth (Variables|/Game/UrnBased/Blueprints/Tile.Tile_C|GetCube _array_element) true)))

(fn GetTilesAround
  (params (Radius :type Float%20%28single-precision%29) (Location :type Vector))
  (bind _tilearray (LocalVariables|GetTileArray))
  (bind _sphere (Variables|Default|GetSphere))
  (Components|Activation|SetActive _sphere true false)
  (Components|Sphere|SetSphereRadius _sphere (* Radius 5e+01) true)
  (for _array_element (Collision|GetOverlappingActors _sphere "/Game/UrnBased/Blueprints/Tile.Tile_C" :!class /Script/Engine.PrimitiveComponent)
    (Utilities|Array|Add _tilearray (.AsTile (Utilities|Casting|CastToTile _array_element))))
  (Components|Activation|SetActive (Variables|Default|GetSphere) false true)
  (return _tilearray))