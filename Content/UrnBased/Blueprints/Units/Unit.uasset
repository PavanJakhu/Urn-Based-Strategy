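; Selectable, team-colored unit for turn-based tactical play, with Move, Attack and Defend actions driven by a state variable.
; Move and Attack resize a sphere to find tiles or units in range, highlighting them via custom depth; MoveUnitTo uses AIMoveTo.
; Clicks update the GameMode's selection and trigger attacks on targetable units, which deal damage and refresh the unit card.
; Defend doubles endurance until the next turn begins.
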(event Custom|MoveUnitTo
  (params (Location :type Vector))
  ;[1 1 1] Custom event to move the unit
  (switch Utilities|FlowControl|Switch|SwitchonUnitStates (Variables|Default|GetmyState)
    (:NewEnumerator0
      (AI|AIMoveTo self Location 0 5.0 false))))

(event EventBeginPlay
  (Components|Activation|SetActive (Variables|Default|GetSphere) false false))

(event MouseInput|EventActorOnClicked
  (Utilities|FlowControl|Sequence
    (:then_0
      ;[1 1 1] Attack the next clicked unit
      (if (Variables|Default|GetcanBeTargetted)
        (bind _asgm_urn_based (Utilities|Casting|CastToGM_UrnBased (Game|GetGameMode)))
        (bind _selectedunit (Default|GetSelectedUnit _asgm_urn_based))
        (bind _output_get (Variables|Unit_C|SettargetUnit self _selectedunit))
        (CallFunction|Attack _output_get)))
    (:then_1
      ;[1 1 1] When clicking a unit highlight the tiles and select the new unit
      (bind _asgm_urn_based_2 (Utilities|Casting|CastToGM_UrnBased (Game|GetGameMode)))
      (bind _selectedunit_2 (Default|GetSelectedUnit _asgm_urn_based_2))
      (if (!= _selectedunit_2 0)
        (for _array_element (Variables|Unit_C|GettilesAround _selectedunit_2)
          (Rendering|SetRenderCustomDepth (Variables|/Game/UrnBased/Blueprints/Tile.Tile_C|GetCube _array_element) false))
        (Utilities|Array|Clear (Variables|Unit_C|GettilesAround _selectedunit_2)))
      (Default|SetSelectedUnit _asgm_urn_based_2 self))))

(fn ConstructionScript
  (bind _cylinder (Variables|Default|GetCylinder))
  (Class|UrnUnit|SetStartingStats 10 3 3 10 10 10 10 10 10 10 10 3 1)
  (switch Utilities|FlowControl|Switch|SwitchonTeamColours (Variables|Default|GetmyTeam)
    (:NewEnumerator0
      (Rendering|Material|SetMaterial _cylinder 0 "/Game/StarterContent/Materials/M_Metal_Rust.M_Metal_Rust"))
    (:NewEnumerator1
      (Rendering|Material|SetMaterial _cylinder 0 "/Game/StarterContent/Materials/M_Water_Lake.M_Water_Lake"))
    (:NewEnumerator2
      (Rendering|Material|SetMaterial _cylinder 0 "/Game/StarterContent/Materials/M_Ground_Grass.M_Ground_Grass"))))

(fn GetMyStats
  (return (Variables|Default|GetmyStats)))

(fn OnAttackClicked
  (Variables|Default|SetmyState "NewEnumerator1")
  (bind _myunitstats (CallFunction|GetMyStats))
  (bind _actors (CallFunction|GetObjectsAround (* (.range _myunitstats) 1e+02) "Unit_C"))
  (for _array_element _actors
    (if (not (== _array_element self))
      (bind _asunit (Utilities|Casting|CastToUnit _array_element))
      (Rendering|SetRenderCustomDepth (Variables|Unit_C|GetCylinder _asunit) true)
      (CallFunction|SetCanbeTargetted _asunit true))))

(fn Attack
  (bind _self self)
  (bind _targetunit (Variables|Default|GettargetUnit))
  (CallFunction|GetMyStats _self)
  (Class|UrnUnit|CalculateDamageTaken _targetunit (Utilities|Struct|MakeAttackInfo "ATT_MELEE" 3 _self))
  (bind _asgm_urn_based (Utilities|Casting|CastToGM_UrnBased (Game|GetGameMode)))
  (bind _myunitstats (CallFunction|GetMyStats _targetunit))
  (Development|PrintString (Utilities|String|ToString(Integer) (.hitpoints _myunitstats)))
  (Development|PrintString (Utilities|String|ToString(Integer) (.maxhitpoints _myunitstats)))
  (Default|UpdateTargetUnit (Variables|/Game/UrnBased/Blueprints/GM_UrnBased.GM_UrnBased_C|GetUnitCardRef _asgm_urn_based) _targetunit))

(fn SetCanbeTargetted
  (params (canBeTarget :type Boolean))
  (Variables|Default|SetcanBeTargetted canBeTarget))

(fn OnDefendClicked
  (Variables|Default|SetmyState "NewEnumerator3")
  (Development|PrintString "Set Active Pawn's Endurance to x 2 until it is active again")
  (Variables|Default|SetwasDefending true)
  (Variables|Default|SetmyStats (Utilities|Struct|MakeUnitStats (.hitpoints (Variables|Default|GetmyStats)) (.maxhitpoints (Variables|Default|GetmyStats)) (.speed (Variables|Default|GetmyStats)) (.actionpoints (Variables|Default|GetmyStats)) (.maxactionpoints (Variables|Default|GetmyStats)) (.powerpoints (Variables|Default|GetmyStats)) (.maxpowerpoints (Variables|Default|GetmyStats)) (.prowess (Variables|Default|GetmyStats)) (.accuracy (Variables|Default|GetmyStats)) (.strength (Variables|Default|GetmyStats)) (* (.endurance (Variables|Default|GetmyStats)) 2) (.agility (Variables|Default|GetmyStats)) (.willpower (Variables|Default|GetmyStats)) (.intelligence (Variables|Default|GetmyStats)) (.armour (Variables|Default|GetmyStats)) (.size (Variables|Default|GetmyStats)) (.range (Variables|Default|GetmyStats)))))

(fn OnTurnBegin
  (if (Variables|Default|GetwasDefending)
    (Variables|Default|SetwasDefending false)
    (Variables|Default|SetmyStats (Utilities|Struct|MakeUnitStats (.hitpoints (Variables|Default|GetmyStats)) (.maxhitpoints (Variables|Default|GetmyStats)) (.speed (Variables|Default|GetmyStats)) (.actionpoints (Variables|Default|GetmyStats)) (.maxactionpoints (Variables|Default|GetmyStats)) (.powerpoints (Variables|Default|GetmyStats)) (.maxpowerpoints (Variables|Default|GetmyStats)) (.prowess (Variables|Default|GetmyStats)) (.accuracy (Variables|Default|GetmyStats)) (.strength (Variables|Default|GetmyStats)) (/ (.endurance (Variables|Default|GetmyStats)) 2) (.agility (Variables|Default|GetmyStats)) (.willpower (Variables|Default|GetmyStats)) (.intelligence (Variables|Default|GetmyStats)) (.armour (Variables|Default|GetmyStats)) (.size (Variables|Default|GetmyStats)) (.range (Variables|Default|GetmyStats))))))

(fn OnTurnEnd)

(fn OnMoveClicked
  (Variables|Default|SetmyState "NewEnumerator0")
  (Development|PrintString "OnMoveClicked")
  (bind _asgm_urn_based (Utilities|Casting|CastToGM_UrnBased (Game|GetGameMode)))
  (bind _selectedunit (Default|GetSelectedUnit _asgm_urn_based))
  (bind _myunitstats (CallFunction|GetMyStats _selectedunit))
  (bind _actors (CallFunction|GetObjectsAround _selectedunit (Math|Conversions|ToFloat(Integer) (.speed _myunitstats)) "/Game/UrnBased/Blueprints/Tile.Tile_C"))
  (for _array_element _actors
    (Utilities|Array|Add (Variables|Default|GettilesAround) (.AsTile (Utilities|Casting|CastToTile _array_element)))
    (Rendering|SetRenderCustomDepth (Variables|/Game/UrnBased/Blueprints/Tile.Tile_C|GetCube (.AsTile (Utilities|Casting|CastToTile _array_element))) true)))

(fn GetObjectsAround
  (params (Radius :type Float%20%28single-precision%29) (ClassFilter :type Object%20Class%20Reference))
  (bind _sphere (Variables|Default|GetSphere))
  (bind _overlappingactors (Collision|GetOverlappingActors _sphere ClassFilter :!class /Script/Engine.PrimitiveComponent))
  (Components|Activation|SetActive _sphere true true)
  (Components|Sphere|SetSphereRadius _sphere (* Radius 1e+02) true)
  (for _array_element _overlappingactors
    (Utilities|Array|Add (LocalVariables|GetActorArray) (.AsTile (Utilities|Casting|CastToTile _array_element))))
  (Components|Activation|SetActive (Variables|Default|GetSphere) false true)
  (return _overlappingactors))

(fn GetMyState
  (return (Variables|Default|GetmyState)))